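; BP_Card is a clickable playing card actor that displays a suit and value.
; On BeginPlay it creates one WBP_CardValues widget from its CardSuit and CardValue and assigns it to both Widget1 and Widget2 components.
; Clicking the mesh sets its world pitch to 180 degrees while keeping roll and yaw, turning the card over without animation or toggling back.
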(event `self.ReceiveBeginPlay`
  (bind _returnvalue (`|CreateWidget` "/Game/CardDeck/Card/WBP_CardValues.WBP_CardValues_C" null (`self.CardSuit`) (`self.CardValue`)))
  (`WidgetComponent.SetWidget` (`self.Widget1`) _returnvalue)
  (`WidgetComponent.SetWidget` (`self.Widget2`) _returnvalue))

(event `self.Mesh.OnClicked`
  (params (TouchedComponent :type "PrimitiveComponent Object Reference") (ButtonPressed :type "Key Structure"))
  (bind (_returnvalue_roll _returnvalue_pitch _returnvalue_yaw) (`KismetMathLibrary.BreakRotator` (`SceneComponent.K2_GetComponentRotation` (`self.Mesh`))))
  (`SceneComponent.K2_SetWorldRotation` (`self.Mesh`) (`KismetMathLibrary.MakeRotator` _returnvalue_roll 180.0 _returnvalue_yaw) false false))

(fn `UserConstructionScript`)