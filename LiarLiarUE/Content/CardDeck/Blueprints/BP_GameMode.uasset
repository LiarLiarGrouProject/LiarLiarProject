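; BP_GameMode is a game mode that builds a deck of playing cards when play begins.
; Nested loops over the value and suit lists spawn one BP_Card per combination, passing in its suit and value.
; Each card spawns higher by the card thickness times a running count to form a stack, and is added to the Deck array.
; A Deck shuffle node exists but is unconnected, so the deck stays in spawn order.
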(event `self.ReceiveBeginPlay`
  (for _array_element (`self.Value`)
    (for _array_element_2 (`self.Suits`)
      (bind _returnvalue (`|SpawnActorFromClass` "/Game/CardDeck/Blueprints/BP_Card.BP_Card_C" (`KismetMathLibrary.MakeTransform` (`KismetMathLibrary.MakeVector` 0.0 0.0 (+ 360.0 (* (`self.CardThickness`) (`self.CardCount`))))) "Undefined" "MultiplyWithRoot" null _array_element_2 _array_element null))
      (`KismetArrayLibrary.Array_Add` (`self.Deck`) _returnvalue)
      (`/Engine/EditorBlueprintResources/StandardMacros.IncrementFloat` (`self.CardCount`)))))

(fn `UserConstructionScript`)